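; MQTT client actor that links a tower defense game to a remote server.
; On BeginPlay it connects to a hardcoded broker; Click and Init publish tower and player JSON requests.
; Receive events spawn towers, creeps and projectiles, and update creep targets and HP.
; Creeps and projectiles are tracked by server ID; towers are untracked, TowerDie searches CreepMap, and both creep-map removals use key 0.
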(event `self.ReceiveBeginPlay`
  (`self.CreateClient` (`KismetStringLibrary.Concat_StrStr` "id" (`KismetStringLibrary.Conv_IntToString` (`KismetMathLibrary.RandomInteger` 1000))) "203.204.228.101")
  (`self.Connect` 5))

(event `Click`
  (params (pos :type "Vector Structure"))
  (bind _returnvalue (`WebInterfaceJsonObject.SetString` (`WebInterfaceHelpers.ConstructObject`) "t" "tower"))
  (bind _returnvalue_2 (`WebInterfaceJsonObject.SetString` _returnvalue "a" "C"))
  (bind _returnvalue_3 (`WebInterfaceJsonObject.SetString` _returnvalue_2 "name" "test"))
  (bind _returnvalue_4 (`WebInterfaceJsonObject.SetInteger` (`WebInterfaceHelpers.ConstructObject`) "tid" 0))
  (bind _returnvalue_5 (`WebInterfaceJsonObject.SetNumber` _returnvalue_4 "x" (.x pos)))
  (bind _returnvalue_6 (`WebInterfaceJsonObject.SetNumber` _returnvalue_5 "y" (.y pos)))
  (bind _returnvalue_7 (`WebInterfaceJsonObject.SetObject` _returnvalue_3 "d" _returnvalue_6))
  (bind _returnvalue_8 (`WebInterfaceJsonObject.Stringify` _returnvalue_7))
  (`self.Publish` "td/all/send" _returnvalue_8))

(event `Init`
  (bind _returnvalue (`WebInterfaceJsonObject.SetString` (`WebInterfaceHelpers.ConstructObject`) "t" "player"))
  (bind _returnvalue_2 (`WebInterfaceJsonObject.SetString` _returnvalue "a" "C"))
  (bind _returnvalue_3 (`WebInterfaceJsonObject.SetString` _returnvalue_2 "name" "test"))
  (bind _returnvalue_4 (`WebInterfaceJsonObject.SetString` (`WebInterfaceHelpers.ConstructObject`) "name" "test"))
  (bind _returnvalue_5 (`WebInterfaceJsonObject.SetObject` _returnvalue_3 "d" _returnvalue_4))
  (bind _returnvalue_6 (`WebInterfaceJsonObject.Stringify` _returnvalue_5))
  (`self.Publish` "td/all/send" _returnvalue_6))

(event `self.OnConnected`
  (`self.Subscribe` "td/all/res")
  (`KismetSystemLibrary.PrintString` "IsConnect" true true (struct :`R` 1.0 :`B` 0.163095 :`A` 1.0) 5.0))

(event `self.OnReceiveTowerCreate`
  (params (Msg :type "TowerCreate Structure (by ref)"))
  (bind (_id _x _y) (break `TowerCreate` Msg))
  (`KismetSystemLibrary.PrintString` (`KismetTextLibrary.Conv_TextToString` (`|FormatText` "x {x}, y {y}" _x _y)))
  (`|SpawnActorFromClass` "/Game/Tower/Tower1.Tower1_C" (`KismetMathLibrary.MakeTransform` (`KismetMathLibrary.MakeVector` _x _y 10.0)) "Undefined" "OverrideRootScale" null null))

(event `self.OnReceiveCreepCreate`
  (params (Msg :type "CreepCreate Structure (by ref)"))
  (bind (_id _name _x _y _msd _def_magic _def_physic _hp) (break `CreepCreate` Msg))
  (bind _returnvalue (`KismetMathLibrary.MakeVector` _x _y 10.0))
  (bind _value (`BlueprintMapLibrary.Map_Find` (`self.ClassMap`) _name))
  (if (`KismetSystemLibrary.IsValidClass` _value)
    (bind _returnvalue_2 (`|SpawnActorFromClass` _value (`KismetMathLibrary.MakeTransform` _returnvalue) "Undefined" "OverrideRootScale" null _msd _returnvalue _hp _hp null))
    (`BlueprintMapLibrary.Map_Add` (`self.CreepMap`) _id _returnvalue_2)))

(event `self.OnReceiveCreepMove`
  (params (Msg :type "CreepMove Structure (by ref)"))
  (bind (_id _x _y) (break `CreepMove` Msg))
  (bind (_value _returnvalue) (`BlueprintMapLibrary.Map_Find` (`self.CreepMap`) _id))
  (if _returnvalue
    (set `Creep.TargetPoint` (`KismetMathLibrary.MakeVector` _x _y 10.0) _value)))

(event `self.OnReceiveTowerDie`
  (params (Msg :type "ActorDie Structure (by ref)"))
  (bind _creepmap (`self.CreepMap`))
  (bind (_value _returnvalue) (`BlueprintMapLibrary.Map_Find` _creepmap (`.id` (break `ActorDie` Msg))))
  (if _returnvalue
    (`self.K2_DestroyActor` _value)
    (`BlueprintMapLibrary.Map_Remove` _creepmap)))

(event `self.OnReceiveCreepHp`
  (params (Msg :type "CreepHp Structure (by ref)"))
  (bind (_id _hp) (break `CreepHp` Msg))
  (bind (_value _returnvalue) (`BlueprintMapLibrary.Map_Find` (`self.CreepMap`) _id))
  (if _returnvalue
    (set `Creep.Hp` _hp _value)))

(event `self.OnReceiveCreepDie`
  (params (Msg :type "ActorDie Structure (by ref)"))
  (bind _id (break `ActorDie` Msg))
  (bind _creepmap (`self.CreepMap`))
  (bind (_value _returnvalue) (`BlueprintMapLibrary.Map_Find` _creepmap _id))
  (if _returnvalue
    (`self.K2_DestroyActor` _value)
    (`BlueprintMapLibrary.Map_Remove` _creepmap)
    (`KismetSystemLibrary.PrintString` (`KismetStringLibrary.Concat_StrStr` "remove creep " (`KismetStringLibrary.Conv_IntToString` _id)) true true (struct :`R` 1.0 :`G` 0.163524 :`B` 0.307544 :`A` 1.0))))

(event `self.OnReceiveProjectileCreate`
  (params (Msg :type "ProjctileCreate Structure (by ref)"))
  (bind (_id _owner _radius _target _time_left _x _y _msd) (break `ProjctileCreate` Msg))
  (bind (_value _returnvalue) (`BlueprintMapLibrary.Map_Find` (`self.CreepMap`) _target))
  (if _returnvalue
    (bind _returnvalue_2 (`|SpawnActorFromClass` "/Game/Projectile/proj1.proj1_C" (`KismetMathLibrary.MakeTransform` (`KismetMathLibrary.MakeVector` _x _y 30.0)) "Undefined" "OverrideRootScale" null _msd _value null))
    (`BlueprintMapLibrary.Map_Add` (`self.ProjMap`) _id _returnvalue_2)))

(event `self.OnReceiveProjectileDie`
  (params (Msg :type "ActorDie Structure (by ref)"))
  (bind _id (break `ActorDie` Msg))
  (bind _projmap (`self.ProjMap`))
  (bind (_value _returnvalue) (`BlueprintMapLibrary.Map_Find` _projmap _id))
  (if _returnvalue
    (if (`KismetSystemLibrary.IsValid` _value)
      (`self.K2_DestroyActor` _value))
    (`BlueprintMapLibrary.Map_Remove` _projmap _id)))

(fn `UserConstructionScript`)