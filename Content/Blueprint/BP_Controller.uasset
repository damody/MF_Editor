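; BP_Controller is a player controller that shows the mouse cursor and forwards input to the first BP_TDMqtt actor found in the level.
; Space bar calls that actor's Init.
; A left click traces from the cursor into the world on the Visibility channel, with debug drawing, and passes the hit location to its Click function without checking for a hit.
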(event `self.ReceiveBeginPlay`
  (set `self.bShowMouseCursor` true))

(event `Key|SpaceBar`
  (params (Key :type "Key Structure"))
  (:`Pressed`
    (bind _outactors (`GameplayStatics.GetAllActorsOfClass` "/Game/Blueprint/BP_TDMqtt.BP_TDMqtt_C"))
    (`/Game/Blueprint/BP_TDMqtt.Init` (`|GetArrayItem` _outactors))))

(event `Key|LeftMouseButton`
  (params (Key :type "Key Structure"))
  (bind (_worldlocation _worlddirection) (`self.DeprojectMousePositionToWorld`))
  (:`Pressed`
    (bind _outactors (`GameplayStatics.GetAllActorsOfClass` "/Game/Blueprint/BP_TDMqtt.BP_TDMqtt_C"))
    (bind _outhit (`KismetSystemLibrary.LineTraceSingle` :`Start` _worldlocation :`End` (+ _worldlocation (* _worlddirection 10000.0)) :`TraceChannel` "TraceTypeQuery1" :`DrawDebugType` "ForDuration"))
    (`/Game/Blueprint/BP_TDMqtt.Click` (`|GetArrayItem` _outactors) (`.Location` (`GameplayStatics.BreakHitResult` _outhit)))))

(fn `UserConstructionScript`)